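; Blood Elf player character Blueprint that drives head turning and aim orientation while the character stands idle.
; After the parent Tick, when idle and not falling, it calls UpdateHeadRotation with left and right shuffle montages.
; The result is written to HeadRotation on the AB_BloodElf anim instance.
; That rotation also sets the Aim component's relative rotation, with pitch and roll swapped and the original roll negated.
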(event EventBeginPlay)

(event Collision|EventActorBeginOverlap
  (params (OtherActor :type Actor%20Object%20Reference)))

(event EventTick
  (params (DeltaSeconds :type Float%20%28single-precision%29))
  (|CallParentFunction DeltaSeconds)
  (bind _asab_blood_elf (Utilities|Casting|CastToAB_BloodElf (Components|SkeletalMesh|GetAnimInstance (Variables|Character|GetMesh))))
  (if (and (Variables|Default|GetIsIdle?) (not (AI|Components|NavMovement|IsFalling (Variables|Character|GetCharacterMovement))))
    (bind _headrotation (CallFunction|UpdateHeadRotation "/Game/Player/Model/BloodElf_Normal/Montage/BloodElf_Anim_ShuffleRight__24__Montage.BloodElf_Anim_ShuffleRight__24__Montage" "/Game/Player/Model/BloodElf_Normal/Montage/BloodElf_Anim_ShuffleLeft__23__Montage.BloodElf_Anim_ShuffleLeft__23__Montage"))
    (Variables|/Game/Player/Model/BloodElf_Normal/Animation/AB_BloodElf.AB_BloodElf_C|SetHeadRotation _asab_blood_elf _headrotation)
    (Transformation|SetRelativeRotation (Variables|Default|GetAim) (Math|Rotator|MakeRotator (.pitch (Variables|/Game/Player/Model/BloodElf_Normal/Animation/AB_BloodElf.AB_BloodElf_C|GetHeadRotation _asab_blood_elf)) (* (.roll (Variables|/Game/Player/Model/BloodElf_Normal/Animation/AB_BloodElf.AB_BloodElf_C|GetHeadRotation _asab_blood_elf)) -1.0) (.yaw (Variables|/Game/Player/Model/BloodElf_Normal/Animation/AB_BloodElf.AB_BloodElf_C|GetHeadRotation _asab_blood_elf))) false false)))

(fn ConstructionScript
  (|CallParentFunction))